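; Old_Book is a collectible pickup that triggers the win screen when the player touches it.
; Overlapping Book_Collision with a Player_Character adds to that character's Book variable and destroys the actor.
; It then pauses the game, shows Win_Widget and switches to UI-only input with a visible cursor.
; A yaw-spin for the mesh exists but is disconnected, and Tick is empty.
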(event `self.ReceiveTick`
  (params (DeltaSeconds :type "Float (single-precision)")))

(event `self.Book_Collision.OnComponentBeginOverlap`
  (params (OverlappedComponent :type "PrimitiveComponent Object Reference") (OtherActor :type "Actor Object Reference") (OtherComp :type "PrimitiveComponent Object Reference") (OtherBodyIndex :type Integer) (bFromSweep :type Boolean) (SweepResult :type "HitResult Structure (by ref)"))
  (bind _returnvalue (`GameplayStatics.GetPlayerController` 0))
  (bind _asplayer_character (cast `/Game/Paul/ThirdPersonBP/Blueprints/Player_Character` OtherActor))
  (set `/Game/Paul/ThirdPersonBP/Blueprints/Player_Character.Book` (+ (`/Game/Paul/ThirdPersonBP/Blueprints/Player_Character.Book` _asplayer_character) (`self.Book`)) _asplayer_character)
  (`self.K2_DestroyActor`)
  (`GameplayStatics.SetGamePaused` true)
  (bind _returnvalue_2 (`|CreateWidget` "/Game/Paul/UI/Win_Widget.Win_Widget_C" _returnvalue))
  (`UserWidget.AddToViewport` _returnvalue_2 0)
  (`WidgetBlueprintLibrary.SetInputMode_UIOnlyEx` _returnvalue null)
  (set `PlayerController.bShowMouseCursor` true _returnvalue))

(fn `UserConstructionScript`)