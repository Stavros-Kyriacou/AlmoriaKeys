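; Destructible egg that serves as a kill objective, counting toward the player's victory condition.
; It replays a hatching sound at random intervals and loses clamped health on damage, dying once on a hit taken at zero health.
; Death swaps to the broken mesh, plays sound and particles, and reports AI noise at the player's location.
; It then increments the player's EggKills and calls Victory when all eggs are destroyed.
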(event `self.ReceiveBeginPlay`
  (`self.Hatching_Sound`))

(event `Hatching_Sound`
  (`KismetSystemLibrary.Delay` (`KismetMathLibrary.RandomFloatInRange` 6.0 12.0))
  (if (not (`self.IsDestroyed`))
    (`GameplayStatics.PlaySoundAtLocation` "/Game/Stavros/Audio/EggHatching/SC_Egg_Hatching.SC_Egg_Hatching" (`SceneComponent.K2_GetComponentLocation` (`self.DefaultSceneRoot`)) (struct) 1.0 1.0 0.0 null null null)
    (`self.Hatching_Sound`)))

(event `self.ReceiveAnyDamage`
  (params (Damage :type "Float (single-precision)") (DamageType :type "DamageType Object Reference") (InstigatedBy :type "Controller Object Reference") (DamageCauser :type "Actor Object Reference"))
  ;[1 1 1] Check if health is above 0
  (if (> (`self.Health`) 0.0)
    ;[1 1 1] Subtract damage from health
    (set `self.Health` (`KismetMathLibrary.FClamp` (- (`self.Health`) Damage)))
    (else
      ;[1 1 1] If out of health, call the death function
      (`/Engine/EditorBlueprintResources/StandardMacros.DoOnce` false
        (:`Completed`
          (`self.Death`))))))

(event `Death`
  (bind _returnvalue (`GameplayStatics.GetPlayerCharacter` 0))
  (bind _playerreference (`self.PlayerReference`))
  (bind _playerreference_2 (`self.PlayerReference`))
  ;[1 1 1] Egg death function
  ;;[1 1 1] Hide the Egg mesh, show the Broken Egg mesh
  (`SceneComponent.SetVisibility` (`self.Egg`) false false)
  (`SceneComponent.SetVisibility` (`self.Egg_Broken`) true false)
  ;;[1 1 1] Play sound effect
  (`GameplayStatics.PlaySoundAtLocation` "/Game/Stavros/Audio/EggDestruction/SC_Egg_Destruction.SC_Egg_Destruction" (`SceneComponent.K2_GetComponentLocation` (`self.DefaultSceneRoot`)) (struct) 1.0 1.0 0.0 null null null)
  (`AISense_Hearing.ReportNoiseEvent` (`self.K2_GetActorLocation` _returnvalue) 1.0 _returnvalue 0.0 "Noise")
  ;;[1 1 1] Activate particle system
  (`ActorComponent.Activate` (`self.ParticleSystem`) false)
  (set `/Game/Stavros/Blueprints/FirstPersonCharacter_Exterminator.EggKills` (+ (`/Game/Stavros/Blueprints/FirstPersonCharacter_Exterminator.EggKills` _playerreference) 1) _playerreference)
  (if (>= (`/Game/Stavros/Blueprints/FirstPersonCharacter_Exterminator.EggKills` _playerreference_2) (`/Game/Stavros/Blueprints/FirstPersonCharacter_Exterminator.NumberOfEggs` _playerreference_2))
    (`/Game/Stavros/Blueprints/FirstPersonCharacter_Exterminator.Victory` (`self.PlayerReference`))))

(fn `UserConstructionScript`)