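; BP_Ammo_Crate is an interactable ammo crate that shows a text prompt while the player stands near it.
; Overlap events on BoxTrigger filter for FirstPersonCharacter_Exterminator, set InTrigger, and toggle the TextRender's visibility to match.
; The Interact event calls Reload, which is an empty stub in this graph, so no ammo is granted here.
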(event `/Game/Stavros/Blueprints/BP_Interfaces.Interact`
  (`self.Reload`))

(event `Reload`)

(event `self.BoxTrigger.OnComponentBeginOverlap`
  (params (OverlappedComponent :type "PrimitiveComponent Object Reference") (OtherActor :type "Actor Object Reference") (OtherComp :type "PrimitiveComponent Object Reference") (OtherBodyIndex :type Integer) (bFromSweep :type Boolean) (SweepResult :type "HitResult Structure (by ref)"))
  ;[1 1 1] Interact interface message
  (cast `/Game/Stavros/Blueprints/FirstPersonCharacter_Exterminator` OtherActor)
  (set `self.InTrigger` true)
  ;;[1 1 1] Check if the player is in range of the box trigger and set the visibility of the text renderer
  (if (`self.InTrigger`) :!label _label
    (`SceneComponent.SetVisibility` (`self.TextRender`) true false)
    (else
      (`SceneComponent.SetVisibility` (`self.TextRender`) false false))))

(event `self.BoxTrigger.OnComponentEndOverlap`
  (params (OverlappedComponent :type "PrimitiveComponent Object Reference") (OtherActor :type "Actor Object Reference") (OtherComp :type "PrimitiveComponent Object Reference") (OtherBodyIndex :type Integer))
  ;[1 1 1] Interact interface message
  (cast `/Game/Stavros/Blueprints/FirstPersonCharacter_Exterminator` OtherActor)
  (set `self.InTrigger` false)
  (goto _label))

(fn `UserConstructionScript`)