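; AI creature that roams the level, chases the Exterminator player on sight and calls the player's Death on trigger overlap.
; A looping timer picks random navmesh roam points, gated by fleeing, chasing and moving flags.
; It takes damage only while chasing; at the flee threshold it stops roaming and moves to a random offset around the player.
; Reaching that point resets health and resumes roaming, while failed flee moves retry.
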(event `self.ReceiveAnyDamage`
  (params (Damage :type "Float (single-precision)") (DamageType :type "DamageType Object Reference") (InstigatedBy :type "Controller Object Reference") (DamageCauser :type "Actor Object Reference"))
  ;[1 1 1] only deal damage to the creature if it is chaing player
  (if (`self.IsChasing`)
    ;[1 1 1] Deal damage to creature
    (set `self.Health` (- (`self.Health`) Damage))
    ;[1 1 1] if enough damage has been done. stop roaming and begin fleeing
    (if (<= (`self.Health`) (`self.FleeThreshhold`))
      (`self.STOP Roaming`)
      (set `self.IsFleeing` true)
      (`self.Fleeing`))))

(event `Fleeing`
  (bind (_returnvalue_x _returnvalue_y _returnvalue_z) (`KismetMathLibrary.BreakVector` (`SceneComponent.K2_GetComponentLocation` (`Character.CapsuleComponent` (`GameplayStatics.GetPlayerCharacter` 0)))))
  (`|AIMoveTo` self (`KismetMathLibrary.MakeVector` (+ _returnvalue_x (`KismetMathLibrary.RandomFloatInRange` -1000.0 1000.0)) (+ _returnvalue_y (`KismetMathLibrary.RandomFloatInRange` -1000.0 1000.0)) _returnvalue_z) null :!label _label
    (:`OnSuccess`
      ;[1 1 1] on success, reset health and go back to roaming
      (set `self.IsFleeing` false)
      (set `self.IsMoving` false)
      (set `self.Health` 100.0)
      (`self.Roaming`))
    (:`OnFail`
      (goto _label))))

(event `self.PawnSensing.OnSeePawn`
  (params (Pawn :type "Pawn Object Reference"))
  ;[1 1 1] only chase player if it isnt fleeing from player
  (if (not (`self.IsFleeing`))
    (set `self.IsChasing` true)
    ;[1 1 1] move to player location
    (bind _asfirst_person_character_exterminator (cast `/Game/Stavros/Blueprints/FirstPersonCharacter_Exterminator` Pawn))
    (`|AIMoveTo` self (0.0 0.0 0.0) _asfirst_person_character_exterminator
      (:`then`
        ;[1 1 1] while chasing, stop roaming
        (set `self.IsChasing` true))
      (:`OnSuccess`
        ;[1 1 1] if it reaches the player or cant move to the player, it starts roaming again (player is likely dead if it reaches them anyway
        (set `self.IsChasing` false :!label _label_2))
      (:`OnFail`
        (goto _label_2)))))

(event `STOP Roaming`
  (`KismetSystemLibrary.K2_ClearAndInvalidateTimerHandle` (stale `Roaming` _returnvalue)))

(event `Roaming`
  ;[1 1 1] Loop event every second
  (bind _returnvalue (`KismetSystemLibrary.K2_SetTimerDelegate` (delegate `Roaming`) 1.0 true))
  ;[1 1 1] Only move to new roam location if not fleeing, not chasing and not moving
  (if (`self.IsFleeing`)
    _
    (elif (`self.IsChasing`)
      _
      (elif (not (`self.IsMoving`))
        (`|AIMoveTo` self (`NavigationSystemV1.K2_GetRandomLocationInNavigableRadius` (`self.K2_GetActorLocation`) 1000.0 null null) null
          (:`then`
            ;[1 1 1] While moving to new location, set is moving to true so that it doesnt look for new move to locations
            (set `self.IsMoving` true))
          (:`OnSuccess`
            ;[1 1 1] Once it reaches location or cant reach location, set moving to false so it can look for a new location
            (set `self.IsMoving` false :!label _label_3))
          (:`OnFail`
            (goto _label_3)))))))

(event `self.ReceiveBeginPlay`
  (`self.Roaming`))

(event `self.PlayerDeathTrigger.OnComponentBeginOverlap`
  (params (OverlappedComponent :type "PrimitiveComponent Object Reference") (OtherActor :type "Actor Object Reference") (OtherComp :type "PrimitiveComponent Object Reference") (OtherBodyIndex :type Integer) (bFromSweep :type Boolean) (SweepResult :type "HitResult Structure (by ref)"))
  (bind _asfirst_person_character_exterminator (cast `/Game/Stavros/Blueprints/FirstPersonCharacter_Exterminator` OtherActor))
  (`/Game/Stavros/Blueprints/FirstPersonCharacter_Exterminator.Death` _asfirst_person_character_exterminator))

(fn `UserConstructionScript`
  (`SceneComponent.K2_AttachToComponent` (`self.FP_Gun`) (`self.Mesh2P`) "GripPoint" "SnapToTarget" "SnapToTarget" "SnapToTarget" true))