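; Interactable vent grate that the exterminator player character can open from either side.
; Front and back trigger boxes track whether the player is in range and toggle that side's interaction message on overlap.
; The interface Interact event calls the open logic, which, when in range, destroys both triggers, plays a sound, and after a short delay slides the grate along Y and Z with a timeline.
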(event `/Game/Stavros/Blueprints/BP_Interfaces.Interact`
  ;[1 1 1] Uses the interface blueprint to call the grate open function
  (`self.Grate_Open`))

(event `Grate_Open`
  ;[1 1 1] Open vent grate
  ;;[1 1 1] Check if in range of either trigger box
  (if (or (`self.InTriggerFront`) (`self.InTriggerBack`))
    ;;[1 1 1] Destroy trigger box to stop generating overlap events and making the interaction message appear
    (`ActorComponent.K2_DestroyComponent` (`self.TriggerBoxFront`))
    (`ActorComponent.K2_DestroyComponent` (`self.TriggerBoxBack`))
    (`GameplayStatics.PlaySoundAtLocation` "/Game/Stavros/Audio/GrateOpen/Grate_Open_1.Grate_Open_1" (`SceneComponent.K2_GetComponentLocation` (`self.VentGrate`)) (struct) 1.0 1.0 0.0 null null null)
    (`KismetSystemLibrary.Delay` 0.2)
    ;;[1 1 1] Timeline graph that changes a value over time, used to generate X and Y values
    (bind (_direction _ventopenamount) (`Timeline|VentOpen`)
      (:`Update`
        ;;[1 1 1] Set new location of vent grate
        (`SceneComponent.K2_SetRelativeLocation` (`self.VentGrate`) (`KismetMathLibrary.MakeVector` 0.0 (* _ventopenamount -180.0) (* _ventopenamount 24.0)) false false)))))

(event `self.TriggerBoxFront.OnComponentBeginOverlap`
  (params (OverlappedComponent :type "PrimitiveComponent Object Reference") (OtherActor :type "Actor Object Reference") (OtherComp :type "PrimitiveComponent Object Reference") (OtherBodyIndex :type Integer) (bFromSweep :type Boolean) (SweepResult :type "HitResult Structure (by ref)"))
  ;[1 1 1] Toggle front interaction message if inside box trigger
  (cast `/Game/Stavros/Blueprints/FirstPersonCharacter_Exterminator` OtherActor)
  (set `self.InTriggerFront` true)
  (if (`self.InTriggerFront`) :!label _label
    (`SceneComponent.ToggleVisibility` (`self.InterfaceMessageFront`) false)
    (else
      (`SceneComponent.ToggleVisibility` (`self.InterfaceMessageFront`) false))))

(event `self.TriggerBoxFront.OnComponentEndOverlap`
  (params (OverlappedComponent :type "PrimitiveComponent Object Reference") (OtherActor :type "Actor Object Reference") (OtherComp :type "PrimitiveComponent Object Reference") (OtherBodyIndex :type Integer))
  ;[1 1 1] Toggle front interaction message if inside box trigger
  (cast `/Game/Stavros/Blueprints/FirstPersonCharacter_Exterminator` OtherActor)
  (set `self.InTriggerFront` false)
  (goto _label))

(event `self.TriggerBoxBack.OnComponentBeginOverlap`
  (params (OverlappedComponent :type "PrimitiveComponent Object Reference") (OtherActor :type "Actor Object Reference") (OtherComp :type "PrimitiveComponent Object Reference") (OtherBodyIndex :type Integer) (bFromSweep :type Boolean) (SweepResult :type "HitResult Structure (by ref)"))
  ;[1 1 1] Toggle back interaction message if inside box trigger
  (cast `/Game/Stavros/Blueprints/FirstPersonCharacter_Exterminator` OtherActor)
  (set `self.InTriggerBack` true)
  (if (`self.InTriggerBack`) :!label _label_2
    (`SceneComponent.ToggleVisibility` (`self.InterfaceMessageBack`) false)
    (else
      (`SceneComponent.ToggleVisibility` (`self.InterfaceMessageBack`) false))))

(event `self.TriggerBoxBack.OnComponentEndOverlap`
  (params (OverlappedComponent :type "PrimitiveComponent Object Reference") (OtherActor :type "Actor Object Reference") (OtherComp :type "PrimitiveComponent Object Reference") (OtherBodyIndex :type Integer))
  ;[1 1 1] Toggle back interaction message if inside box trigger
  (cast `/Game/Stavros/Blueprints/FirstPersonCharacter_Exterminator` OtherActor)
  (set `self.InTriggerBack` false)
  (goto _label_2))

(fn `UserConstructionScript`)