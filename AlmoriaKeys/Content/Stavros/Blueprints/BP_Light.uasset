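; BP_Light is a light actor whose spotlight, bulb material and buzzing sound follow the on/off state of its connected switch.
; BeginPlay applies that state so lights can start lit.
; Separate Light_Toggle and Sound_Toggle events re-read the switch to update visuals and audio, with a flag preventing duplicate buzz sounds.
; A Location event prints the actor's root position for debugging.
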(event `self.ReceiveBeginPlay`
  (bind _lightmesh (`self.LightMesh`))
  (bind _isswitchon (`/Game/Stavros/Blueprints/BP_Light_Switch.IsSwitchOn` (`self.ConnectedSwitch`)))
  ;[1 1 1] Same as light toggle function but updates the state when the level starts so that you can have lights that begin on if needed
  (`SceneComponent.SetVisibility` (`self.SpotLight`) _isswitchon false)
  (if _isswitchon
    (bind _returnvalue (`GameplayStatics.SpawnSoundAtLocation` "/Game/Stavros/Audio/LightSwitch/SC_Light_Bulb_Buzzing_Cue.SC_Light_Bulb_Buzzing_Cue" (`SceneComponent.K2_GetComponentLocation` (`self.DefaultSceneRoot`)) (struct) 1.0 1.0 0.0 null null))
    (set `self.BuzzingSound` _returnvalue)
    (set `self.IsPlayingBuzzingSound` true)
    (`PrimitiveComponent.SetMaterial` _lightmesh 0 "/Game/Stavros/Materials/M_Light_On.M_Light_On")
    (else
      (`PrimitiveComponent.SetMaterial` _lightmesh 0 "/Game/Stavros/Materials/M_Light_Off.M_Light_Off"))))

(event `Light_Toggle`
  (bind _lightmesh (`self.LightMesh`))
  (bind _isswitchon (`/Game/Stavros/Blueprints/BP_Light_Switch.IsSwitchOn` (`self.ConnectedSwitch`)))
  ;[1 1 1] Light toggle function
  ;;[1 1 1] Set the visibility of the light to the state of the switch.
  ;; switch on -> light on
  ;; switch off -> light off
  (`SceneComponent.SetVisibility` (`self.SpotLight`) _isswitchon false)
  ;;[1 1 1] Changes the material of the light to remove the emissive colour when it is off
  (if _isswitchon
    (`PrimitiveComponent.SetMaterial` _lightmesh 0 "/Game/Stavros/Materials/M_Light_On.M_Light_On")
    (else
      (`PrimitiveComponent.SetMaterial` _lightmesh 0 "/Game/Stavros/Materials/M_Light_Off.M_Light_Off"))))

(event `Location`
  ;[1 1 1] Light toggle function
  (`KismetSystemLibrary.PrintString` (`KismetStringLibrary.Conv_VectorToString` (`SceneComponent.K2_GetComponentLocation` (`self.DefaultSceneRoot`)))))

(event `Sound_Toggle`
  (if (`/Game/Stavros/Blueprints/BP_Light_Switch.IsSwitchOn` (`self.ConnectedSwitch`))
    (if (not (`self.IsPlayingBuzzingSound`))
      (bind _returnvalue (`GameplayStatics.SpawnSoundAtLocation` "/Game/Stavros/Audio/LightSwitch/SC_Light_Bulb_Buzzing_Cue.SC_Light_Bulb_Buzzing_Cue" (`SceneComponent.K2_GetComponentLocation` (`self.DefaultSceneRoot`)) (struct) 1.0 1.0 0.0 null null))
      (set `self.BuzzingSound` _returnvalue)
      (set `self.IsPlayingBuzzingSound` true))
    (elif (`self.IsPlayingBuzzingSound`)
      (`/Engine/EditorBlueprintResources/StandardMacros.IsValid` (`self.BuzzingSound`)
        (:`Is Valid`
          _)
        (:`Is Not Valid`
          (bind _returnvalue_2 (`GameplayStatics.CreateSound2D` "/Game/Stavros/Audio/LightSwitch/SC_Light_Bulb_Buzzing_Cue.SC_Light_Bulb_Buzzing_Cue" 1.0 1.0 0.0 null))
          (set `self.BuzzingSound` _returnvalue_2)))
      (`AudioComponent.Stop` (`self.BuzzingSound`))
      (set `self.IsPlayingBuzzingSound` false))))

(fn `UserConstructionScript`)