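; Electricity box switch that the player uses to unlock and open a linked door (MyDoor).
; The first interaction inside BoxTrigger swings the box open; the next flicks the switch once, calling OpenDoor and changing the box material.
; Trigger overlaps toggle the text prompt while the door is closed.
; A self-recalling delay plays random spark bursts with sound until the door opens, alongside leftover experimental timeline logic.
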(event `Stop Timeline`
  (bind _particlesystem (`self.ParticleSystem`))
  ;[1 1 1] experimental
  (bind (_direction _newtrack_0) (`Timeline|Timeline_Sparks` :!via `Stop`)
    (:`Update`
      (if (`/Game/Stavros/Blueprints/BP_Door.IsOpen` (`self.MyDoor`))
        (`self.Stop Timeline`)
        (elif (>= _newtrack_0 0.99)
          (`ActorComponent.Activate` _particlesystem false)
          (`/Engine/EditorBlueprintResources/StandardMacros.DoOnce` false
            (:`Completed`
              (`GameplayStatics.PlaySoundAtLocation` "/Game/Stavros/Audio/Sparks/SC_Sparks.SC_Sparks" (`SceneComponent.K2_GetComponentLocation` (`self.DefaultSceneRoot`)) (struct) 1.0 1.0 0.0 null null null)
              (`self.Reset`)
              (`self.Sparks`)))
          (else
            (`ActorComponent.Deactivate` _particlesystem)))))))

(event `Reset`
  ;[1 1 1] experimental
)

(event `self.ReceiveBeginPlay`
  (`self.Sparks`))

(event `Sparks`
  (bind _particlesystem (`self.ParticleSystem`))
  ;[1 1 1] Spark effect + sound
  (`KismetSystemLibrary.Delay` (`KismetMathLibrary.RandomFloatInRange` 5.0 10.0))
  (if (not (`/Game/Stavros/Blueprints/BP_Door.IsOpen` (`self.MyDoor`)))
    (`ActorComponent.Activate` _particlesystem false)
    (`GameplayStatics.PlaySoundAtLocation` "/Game/Stavros/Audio/Sparks/SC_Sparks.SC_Sparks" (`SceneComponent.K2_GetComponentLocation` (`self.DefaultSceneRoot`)) (struct) 1.0 1.0 0.0 null null null)
    (`KismetSystemLibrary.Delay` 0.15)
    (`ActorComponent.Deactivate` _particlesystem)
    (`self.Sparks`)))

(event `/Game/Stavros/Blueprints/BP_Interfaces.Interact`
  ;[1 1 1] Executes the unlock door function when the interact blueprint calls it
  ;;[1 1 1] Check if the box is open. Only call the unlock door function if the electricity box has been opened
  (if (`self.IsDoorOpen`)
    (`self.Unlock_Door`)
    (else
      (`self.Open_Electricy_Box`))))

(event `Open_Electricy_Box`
  ;[1 1 1] Swing open the door, play sound effect and change text on message
  (if (`self.InTrigger`)
    (`SkeletalMeshComponent.PlayAnimation` (`self.SkeletalMesh`) "/Game/Stavros/Models/ElectricityBox/ElectricityBox_Rig_Anim_ElectricityBox_Rig_Door_Open.ElectricityBox_Rig_Anim_ElectricityBox_Rig_Door_Open" false)
    (`GameplayStatics.PlaySoundAtLocation` "/Game/Stavros/Audio/DoorOpen01.DoorOpen01" (`SceneComponent.K2_GetComponentLocation` (`self.DefaultSceneRoot`)) (struct) 1.0 1.0 0.0 null null null)
    (`TextRenderComponent.K2_SetText` (`self.TextRender`) (`|FormatText` "Press 'E' to unlock door"))
    (set `self.IsDoorOpen` true)))

(event `Unlock_Door`
  (bind _mydoor (`self.MyDoor`))
  ;[1 1 1] Unlock the door, executes the open door function from door blueprint
  ;;[1 1 1] Only flick switch once
  (if (not (`self.IsSwitchOpen`))
    ;;[1 1 1] When the player interacts with the switch, check if they are in the box trigger, if they are, unlock the door and call the open door function from the Door blueprint
    (if (`self.InTrigger`)
      (set `/Game/Stavros/Blueprints/BP_Door.IsLocked` false _mydoor)
      (`/Game/Stavros/Blueprints/BP_Door.Open_Door` _mydoor)
      ;;[1 1 1] Door open animation
      (`SkeletalMeshComponent.PlayAnimation` (`self.SkeletalMesh`) "/Game/Stavros/Models/ElectricityBox/ElectricityBox_Rig_Anim_ElectricityBox_Rig_Switches_On.ElectricityBox_Rig_Anim_ElectricityBox_Rig_Switches_On" false)
      (`GameplayStatics.PlaySoundAtLocation` "/Game/Stavros/Audio/LightSwitch/SC_Toggle_Switch.SC_Toggle_Switch" (`SceneComponent.K2_GetComponentLocation` (`self.DefaultSceneRoot`)) (struct) 1.0 1.0 0.0 null null null)
      (`PrimitiveComponent.SetMaterial` (`self.SkeletalMesh`) 0 "/Game/Stavros/Materials/M_Electricty_Box_On.M_Electricty_Box_On")
      ;;[1 1 1] Turn off the text renderer
      (`SceneComponent.SetVisibility` (`self.TextRender`) false false)
      (set `self.IsSwitchOpen` true))))

(event `self.BoxTrigger.OnComponentBeginOverlap`
  (params (OverlappedComponent :type "PrimitiveComponent Object Reference") (OtherActor :type "Actor Object Reference") (OtherComp :type "PrimitiveComponent Object Reference") (OtherBodyIndex :type Integer) (bFromSweep :type Boolean) (SweepResult :type "HitResult Structure (by ref)"))
  ;[1 1 1] Interact interface message
  (cast `/Game/Stavros/Blueprints/FirstPersonCharacter_Exterminator` OtherActor)
  ;;[1 1 1] Check if player is in the box trigger
  (set `self.InTrigger` true)
  ;;[1 1 1] If the door is already open, don't show the interact message
  (if (not (`/Game/Stavros/Blueprints/BP_Door.IsOpen` (`self.MyDoor`))) :!label _label
    ;;[1 1 1] Check if the player is in range of the box trigger and set the visibility of the text renderer
    (if (`self.InTrigger`)
      (`SceneComponent.SetVisibility` (`self.TextRender`) true false)
      (else
        (`SceneComponent.SetVisibility` (`self.TextRender`) false false)))))

(event `self.BoxTrigger.OnComponentEndOverlap`
  (params (OverlappedComponent :type "PrimitiveComponent Object Reference") (OtherActor :type "Actor Object Reference") (OtherComp :type "PrimitiveComponent Object Reference") (OtherBodyIndex :type Integer))
  ;[1 1 1] Interact interface message
  (cast `/Game/Stavros/Blueprints/FirstPersonCharacter_Exterminator` OtherActor)
  ;;[1 1 1] Check if player is in the box trigger
  (set `self.InTrigger` false)
  (goto _label))

(fn `UserConstructionScript`)