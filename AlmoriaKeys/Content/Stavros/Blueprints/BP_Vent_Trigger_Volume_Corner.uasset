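; Corner vent trigger volume that marks the Exterminator player as inside a vent and hides them from the creature's senses.
; Two box components each track player overlap with their own flag.
; While either flag is set, the player's InVent is true and the referenced creature's PawnSensing updates are disabled.
; Only when the player has left both boxes are InVent cleared and sensing re-enabled.
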(event `self.Box.OnComponentBeginOverlap`
  (params (OverlappedComponent :type "PrimitiveComponent Object Reference") (OtherActor :type "Actor Object Reference") (OtherComp :type "PrimitiveComponent Object Reference") (OtherBodyIndex :type Integer) (bFromSweep :type Boolean) (SweepResult :type "HitResult Structure (by ref)"))
  (bind _asfirst_person_character_exterminator (cast `/Game/Stavros/Blueprints/FirstPersonCharacter_Exterminator` OtherActor))
  (set `self.InA` true)
  (if (or (`self.InA`) (`self.InB`))
    (set `/Game/Stavros/Blueprints/FirstPersonCharacter_Exterminator.InVent` true _asfirst_person_character_exterminator)
    (`PawnSensingComponent.SetSensingUpdatesEnabled` (`/Game/Stavros/Blueprints/BP_AI_Creature.PawnSensing` (`self.Creature_Reference`)) false)))

(event `self.Box.OnComponentEndOverlap`
  (params (OverlappedComponent :type "PrimitiveComponent Object Reference") (OtherActor :type "Actor Object Reference") (OtherComp :type "PrimitiveComponent Object Reference") (OtherBodyIndex :type Integer))
  (bind _asfirst_person_character_exterminator (cast `/Game/Stavros/Blueprints/FirstPersonCharacter_Exterminator` OtherActor))
  (set `self.InA` false)
  (if (not (or (`self.InA`) (`self.InB`)))
    (set `/Game/Stavros/Blueprints/FirstPersonCharacter_Exterminator.InVent` false _asfirst_person_character_exterminator)
    (`PawnSensingComponent.SetSensingUpdatesEnabled` (`/Game/Stavros/Blueprints/BP_AI_Creature.PawnSensing` (`self.Creature_Reference`)) true)))

(event `self.Box1.OnComponentBeginOverlap`
  (params (OverlappedComponent :type "PrimitiveComponent Object Reference") (OtherActor :type "Actor Object Reference") (OtherComp :type "PrimitiveComponent Object Reference") (OtherBodyIndex :type Integer) (bFromSweep :type Boolean) (SweepResult :type "HitResult Structure (by ref)"))
  (bind _asfirst_person_character_exterminator (cast `/Game/Stavros/Blueprints/FirstPersonCharacter_Exterminator` OtherActor))
  (set `self.InB` true)
  (if (or (`self.InA`) (`self.InB`))
    (set `/Game/Stavros/Blueprints/FirstPersonCharacter_Exterminator.InVent` true _asfirst_person_character_exterminator)
    (`PawnSensingComponent.SetSensingUpdatesEnabled` (`/Game/Stavros/Blueprints/BP_AI_Creature.PawnSensing` (`self.Creature_Reference`)) false)))

(event `self.Box1.OnComponentEndOverlap`
  (params (OverlappedComponent :type "PrimitiveComponent Object Reference") (OtherActor :type "Actor Object Reference") (OtherComp :type "PrimitiveComponent Object Reference") (OtherBodyIndex :type Integer))
  (bind _asfirst_person_character_exterminator (cast `/Game/Stavros/Blueprints/FirstPersonCharacter_Exterminator` OtherActor))
  (set `self.InB` false)
  (if (not (or (`self.InA`) (`self.InB`)))
    (set `/Game/Stavros/Blueprints/FirstPersonCharacter_Exterminator.InVent` false _asfirst_person_character_exterminator)
    (`PawnSensingComponent.SetSensingUpdatesEnabled` (`/Game/Stavros/Blueprints/BP_AI_Creature.PawnSensing` (`self.Creature_Reference`)) true)))

(fn `UserConstructionScript`)