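; BP_Door is a sliding double door that opens when its Open_Door event is called, unless it is locked or already open.
; Opening plays a slide sound at the door and runs the DoorOpen timeline, which moves the left and right panels apart along relative X.
; IsOpen is set during the timeline updates, and the graph has no closing logic.
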(event `Open_Door`
  ;[1 1 1] Open Door Function
  ;;[1 1 1] Check if door and is locked and if door is open. Door won't open if it is locked, plays sound effect only if the door hasn't been opened.
  (if (`self.IsLocked`)
    _
    (elif (not (`self.IsOpen`))
      (`GameplayStatics.PlaySoundAtLocation` "/Game/Stavros/Audio/DoorSLide/Door_Slide_1.Door_Slide_1" (`SceneComponent.K2_GetComponentLocation` (`self.DefaultSceneRoot`)) (struct) 1.0 1.0 0.0 null null null)
      ;;[1 1 1] Door open movement speed
      (bind (_direction _dooropenamount) (`Timeline|Door Open`)
        (:`Update`
          ;;[1 1 1] Open movement amount
          (`|ExecutionSequence`
            (:`then_0`
              ;;[1 1 1] Set location of movement
              (`SceneComponent.K2_SetRelativeLocation` (`self.LeftDoor`) (`KismetMathLibrary.MakeVector` (* _dooropenamount 110.0)) false false)
              ;;[1 1 1] Set door to open
              (set `self.IsOpen` true))
            (:`then_1`
              (`SceneComponent.K2_SetRelativeLocation` (`self.RightDoor`) (`KismetMathLibrary.MakeVector` (* _dooropenamount -110.0)) false false))))))))

(fn `UserConstructionScript`)