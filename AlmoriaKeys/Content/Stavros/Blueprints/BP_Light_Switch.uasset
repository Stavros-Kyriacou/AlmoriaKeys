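; BP_Light_Switch is an interactable wall switch that toggles the level's lights, starting in the pose set by IsSwitchOn.
; A trigger box tracks whether the exterminator player is in range and shows or hides the interact message.
; An in-range toggle flips the state, plays the switch animation and sound, then calls LightToggle and SoundToggle on every BP_Light, leaving any switch-to-light matching to the lights.
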(event `self.ReceiveBeginPlay`
  (bind _skeletalmesh (`self.SkeletalMesh`))
  (if (`self.IsSwitchOn`)
    (`SkeletalMeshComponent.PlayAnimation` _skeletalmesh "/Game/Stavros/Models/LightSwitch/LightSwitch_Anim_On.LightSwitch_Anim_On" false)
    (else
      (`SkeletalMeshComponent.PlayAnimation` _skeletalmesh "/Game/Stavros/Models/LightSwitch/LightSwitch_Anim_Off.LightSwitch_Anim_Off" false))))

(event `/Game/Stavros/Blueprints/BP_Interfaces.Interact`
  (`self.Light_Switch_Toggle`))

(event `Light_Switch_Toggle`
  (bind _skeletalmesh (`self.SkeletalMesh`))
  ;[1 1 1] Only let player toggle switch if they are in range
  (if (`self.InTrigger`)
    ;[1 1 1] Play animation depending on if switch is on or off
    (if (`self.IsSwitchOn`)
      (set `self.IsSwitchOn` false)
      (`SkeletalMeshComponent.PlayAnimation` _skeletalmesh "/Game/Stavros/Models/LightSwitch/LightSwitch_Anim_Off.LightSwitch_Anim_Off" false)
      ;[1 1 1] Play sound cue
      (`GameplayStatics.PlaySoundAtLocation` "/Game/Stavros/Audio/LightSwitch/SC_Toggle_Switch.SC_Toggle_Switch" (`SceneComponent.K2_GetComponentLocation` (`self.DefaultSceneRoot`)) (struct) 1.0 1.0 0.0 null null null)
      (else
        (set `self.IsSwitchOn` true)
        (`SkeletalMeshComponent.PlayAnimation` _skeletalmesh "/Game/Stavros/Models/LightSwitch/LightSwitch_Anim_On.LightSwitch_Anim_On" false)
        ;[1 1 1] Play sound cue
        (`GameplayStatics.PlaySoundAtLocation` "/Game/Stavros/Audio/LightSwitch/SC_Toggle_Switch.SC_Toggle_Switch" (`SceneComponent.K2_GetComponentLocation` (`self.DefaultSceneRoot`)) (struct) 1.0 1.0 0.0 null null null)))
    ;[1 1 1] For each Light BP, call the Light toggle function from the Light BP. This will toggle the lights on/off if it is connected to the switch
    (bind _outactors (`GameplayStatics.GetAllActorsOfClass` "/Game/Stavros/Blueprints/BP_Light.BP_Light_C"))
    (for _array_element _outactors
      (`/Game/Stavros/Blueprints/BP_Light.Light_Toggle` _array_element)
      (`/Game/Stavros/Blueprints/BP_Light.Sound_Toggle` _array_element))))

(event `self.TriggerBox.OnComponentBeginOverlap`
  (params (OverlappedComponent :type "PrimitiveComponent Object Reference") (OtherActor :type "Actor Object Reference") (OtherComp :type "PrimitiveComponent Object Reference") (OtherBodyIndex :type Integer) (bFromSweep :type Boolean) (SweepResult :type "HitResult Structure (by ref)"))
  ;[1 1 1] Interaction message visibility
  (cast `/Game/Stavros/Blueprints/FirstPersonCharacter_Exterminator` OtherActor)
  (set `self.InTrigger` true)
  (if (`self.InTrigger`) :!label _label
    (`SceneComponent.SetVisibility` (`self.InteractMessage`) true false)
    (else
      (`SceneComponent.SetVisibility` (`self.InteractMessage`) false false))))

(event `self.TriggerBox.OnComponentEndOverlap`
  (params (OverlappedComponent :type "PrimitiveComponent Object Reference") (OtherActor :type "Actor Object Reference") (OtherComp :type "PrimitiveComponent Object Reference") (OtherBodyIndex :type Integer))
  ;[1 1 1] Interaction message visibility
  (cast `/Game/Stavros/Blueprints/FirstPersonCharacter_Exterminator` OtherActor)
  (set `self.InTrigger` false)
  (goto _label))

(fn `UserConstructionScript`)